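; Go board piece actor that shows an empty, black or white state and responds to mouse clicks.
; On BeginPlay it binds the mesh's click event and forwards the component and button to HandleClick, which is defined outside this graph.
; UpdateRender reads GetPieceColor, hiding the actor when empty, or setting the material's Color parameter to black or white and unhiding it.
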(event Custom|PieceClickedDispatcher_Event
  (params (TouchedComponent :type Primitive%20Component%20Object%20Reference) (ButtonPressed :type Key%20Structure :default "None"))
  (Class|GoGameBoardPiece|HandleClick TouchedComponent ButtonPressed))

(event EventBeginPlay
  (EventDispatchers|BindEventtoOnClicked (Variables|Default|GetBoardPieceMesh) (delegate Custom|PieceClickedDispatcher_Event)))

(event Collision|EventActorBeginOverlap
  (params (OtherActor :type Actor%20Object%20Reference)))

(event EventTick
  (params (DeltaSeconds :type Float%20%28single-precision%29)))

(event EventUpdateRender
  (bind _boardpiecemesh (Variables|Default|GetBoardPieceMesh))
  (bind _returnvalue (Class|GoGameBoardPiece|GetPieceColor))
  (switch Utilities|FlowControl|Switch|SwitchonEGoGameCellState _returnvalue
    (:Empty
      (Rendering|SetActorHiddenInGame true))
    (:Black
      (Rendering|Material|SetVectorParameterValueonMaterials _boardpiecemesh "Color" "0, 0, 0")
      (Rendering|SetActorHiddenInGame false :!label _label))
    (:White
      (Rendering|Material|SetVectorParameterValueonMaterials _boardpiecemesh "Color" "1.000000,1.000000,1.000000")
      (goto _label))))

(fn ConstructionScript)